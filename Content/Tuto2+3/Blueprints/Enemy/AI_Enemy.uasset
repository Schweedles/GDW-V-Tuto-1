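; AI_Enemy is an enemy pawn that walks toward the level's objective when play begins.
; On BeginPlay, LocateObjective stores the first BP_Objective actor found in the world, then AIMoveTo sends the pawn to it.
; A GetNextWaypoint function increments a waypoint index, but nothing in this Blueprint calls it or uses that index for movement.
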(event `self.ReceiveBeginPlay`
  (`self.Locate Objective`)
  (`|AIMoveTo` self (0.0 0.0 0.0) (`self.Objective`)))

(fn `Get Next Waypoint`
  (returns (Output_Get :type "Array of Actor Object Reference"))
  (set `self.CurrentWaypointIndex` (+ (`self.CurrentWaypointIndex`) 1))
  (return))

(fn `Locate Objective`
  (locals (NewLocalVar :type "/Game/Tuto2+3/Blueprints/BP_Objective Object Reference"))
  (bind _outactors (`GameplayStatics.GetAllActorsOfClass` "/Game/Tuto2+3/Blueprints/BP_Objective.BP_Objective_C"))
  (set `self.Objective` (`|GetArrayItem` _outactors)))

(fn `UserConstructionScript`)